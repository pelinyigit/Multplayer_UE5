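; Player controller Blueprint that saves and loads a player's loadout through a LoadoutSaveGame slot named after the player.
; Loading restores the loadout and inventory arrays, or triggers a save when no slot exists.
; Saving writes only the loadout to a fresh save object and overwrites current inventory with that object's default InventoryItems.
; A separate event builds a four-entry inventory from supplied amounts to make each player's inventory unique.
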(event `LoadGame_Loadout`
  (bind _returnvalue (`GameplayStatics.GetPlayerState` 0))
  (bind _returnvalue_2 (`PlayerState.GetPlayerName` _returnvalue))
  ;[1 1 1] Save and Load System
  (`/Engine/EditorBlueprintResources/StandardMacros.IsValid` _returnvalue
    (:`Is Valid`
      (bind _returnvalue_3 (`GameplayStatics.DoesSaveGameExist` _returnvalue_2))
      (if _returnvalue_3
        (bind _returnvalue_4 (`GameplayStatics.LoadGameFromSlot` _returnvalue_2))
        (bind _asloadout_save_game (cast `/Game/SaveGame/LoadoutSaveGame` _returnvalue_4))
        (set `self.currentLoadoutStruct` (`/Game/SaveGame/LoadoutSaveGame.loadoutItems` _asloadout_save_game))
        (set `self.currentInventoryStruct` (`/Game/SaveGame/LoadoutSaveGame.InventoryItems` _asloadout_save_game))
        (`KismetSystemLibrary.PrintString` (`KismetStringLibrary.Concat_StrStr` "Loaded Player:" _returnvalue_2) true true (struct :`R` 0.29929 :`G` 1.0 :`A` 1.0))
        (else
          (`self.SaveGame_Loadout`))))))

(event `SaveGame_Loadout`
  (bind _returnvalue (`GameplayStatics.GetPlayerState` 0))
  (bind _returnvalue_2 (`PlayerState.GetPlayerName` _returnvalue))
  ;[1 1 1] Save and Load System
  (set `self.isFirstSave` true)
  (bind _returnvalue_3 (`GameplayStatics.CreateSaveGameObject` "/Game/SaveGame/LoadoutSaveGame.LoadoutSaveGame_C"))
  (set `/Game/SaveGame/LoadoutSaveGame.loadoutItems` (`self.currentLoadoutStruct`) _returnvalue_3)
  (set `self.currentInventoryStruct` (`/Game/SaveGame/LoadoutSaveGame.InventoryItems` _returnvalue_3))
  (`/Engine/EditorBlueprintResources/StandardMacros.IsValid` _returnvalue
    (:`Is Valid`
      (`GameplayStatics.SaveGameToSlot` _returnvalue_3 _returnvalue_2)
      (`KismetSystemLibrary.PrintString` (`KismetStringLibrary.Concat_StrStr` "Saved Player Name:" _returnvalue_2) true true (struct :`R` 0.505126 :`G` 1.0 :`B` 0.507957 :`A` 1.0)))))

(event `SetEachPlayerInventory`
  (params (`ItemAmount 1` :type Integer) (ItemAmount2 :type Integer) (ItemAmount3 :type Integer) (ItemAmount4 :type Integer))
  ;[0.6708 0.3018 1] Set Each Player Inventory Unique
  (set `self.currentInventoryStruct` (`|MakeArray` (make `/Game/Loadout/S_LoadoutItems` "Loadout A" `ItemAmount 1`) (make `/Game/Loadout/S_LoadoutItems` "Loadout B" ItemAmount2) (make `/Game/Loadout/S_LoadoutItems` "Loadout C" ItemAmount3) (make `/Game/Loadout/S_LoadoutItems` "Loadout D" ItemAmount4))))

(fn `UserConstructionScript`)